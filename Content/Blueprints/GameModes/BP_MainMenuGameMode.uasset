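; BP_MainMenuGameMode is the game mode for the main menu.
; On BeginPlay it creates the WBP_MainMenu widget for the first player controller, stores it and adds it to the viewport.
; It also switches input to UI only with focus on that widget, shows the mouse cursor and plays the Cartoon Tanks menu song as a 2D sound.
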(event EventBeginPlay
  ;[1 1 1] Comment
  (bind _returnvalue (UserInterface|CreateWidget "/Game/Blueprints/Widgets/WBP_MainMenu.WBP_MainMenu_C" (Game|GetPlayerController 0)))
  (Variables|Default|SetWBP_MainMenu _returnvalue)
  (Input|SetInputModeUIOnly (Game|GetPlayerController 0) (Variables|Default|GetWBP_MainMenu) "DoNotLock" false)
  (UserInterface|Viewport|AddtoViewport (Variables|Default|GetWBP_MainMenu) 0)
  (Audio|PlaySound2D "/Game/Blueprints/Music/SC_CartoonTanksMainMenuSong.SC_CartoonTanksMainMenuSong" 1.0 1.0 0.0 0 0)
  (Variables|/Script/Engine.PlayerController|SetbShowMouseCursor (Game|GetPlayerController 0) true))

(fn ConstructionScript)