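; Player controller that drives a possessed BaseTank pawn through Enhanced Input move, rotate and shoot actions.
; Move and rotate apply frame-scaled, swept local offsets and rotations using the tank's speed values.
; Shooting plays a character-specific montage chosen by cast, spawns the tank's projectile class at its spawn component after a short delay, and uses a DoOnce to block refiring until the montage time elapses.
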(event Input|EnhancedActionEvents|EnhancedInputActionIA_Rotate
  (params (ActionValue :type Float%20%28double-precision%29) (ElapsedSeconds :type Float%20%28double-precision%29) (TriggeredSeconds :type Float%20%28double-precision%29) (InputAction :type Input%20Action%20Object%20Reference :default "/Game/Blueprints/Input/IA_Rotate.IA_Rotate"))
  (bind _basetank (Variables|Default|GetBaseTank))
  ;[1 1 1] Handle the rotate input action
  (bind _output_get (Variables|/Script/CartoonTanks.BaseTank|SetDeltaRotation _basetank (Math|Rotator|MakeRotator (.roll (Variables|/Script/CartoonTanks.BaseTank|GetDeltaRotation (Variables|Default|GetBaseTank))) (.pitch (Variables|/Script/CartoonTanks.BaseTank|GetDeltaRotation (Variables|Default|GetBaseTank))) (* ActionValue (Utilities|Time|GetWorldDeltaSeconds) (Variables|/Script/CartoonTanks.BaseTank|GetTurnSpeed _basetank)))))
  (Transformation|AddActorLocalRotation (Variables|Default|GetBaseTank) _output_get true false))

(event Input|EnhancedActionEvents|EnhancedInputActionIA_Move
  (params (ActionValue :type Float%20%28double-precision%29) (ElapsedSeconds :type Float%20%28double-precision%29) (TriggeredSeconds :type Float%20%28double-precision%29) (InputAction :type Input%20Action%20Object%20Reference :default "/Game/Blueprints/Input/IA_Move.IA_Move"))
  (bind _basetank (Variables|Default|GetBaseTank))
  ;[1 1 1] Handle the move input action
  (bind _output_get (Variables|/Script/CartoonTanks.BaseTank|SetDeltaLocation _basetank (Math|Vector|MakeVector (* ActionValue (Utilities|Time|GetWorldDeltaSeconds) (Variables|/Script/CartoonTanks.BaseTank|GetMoveSpeed _basetank)) (.y (Variables|/Script/CartoonTanks.BaseTank|GetDeltaLocation _basetank)) (.z (Variables|/Script/CartoonTanks.BaseTank|GetDeltaLocation _basetank)))))
  (Transformation|AddActorLocalOffset (Variables|Default|GetBaseTank) _output_get true false))

(event Input|EnhancedActionEvents|EnhancedInputActionIA_Shoot
  (params (ActionValue :type Boolean) (ElapsedSeconds :type Float%20%28double-precision%29) (TriggeredSeconds :type Float%20%28double-precision%29) (InputAction :type Input%20Action%20Object%20Reference :default "/Game/Blueprints/Input/IA_Shoot.IA_Shoot"))
  ;[1 1 1] Handle the shoot input action
  (Utilities|FlowControl|DoOnce false :!label _label
    (:Completed
      (bind _montagetime (CallFunction|GetShotMontageTime))
      (Utilities|FlowControl|Delay 0.25)
      (CallFunction|SpawnProjectile)
      (Utilities|FlowControl|Delay (- _montagetime 0.25))
      (goto _label Reset))))

(event EventPossess
  (params (PossessedPawn :type Pawn%20Object%20Reference))
  ;[1 1 1] Set the Tank Base reference on possession of the pawn
  (bind _asbase_tank (Utilities|Casting|CastToBaseTank PossessedPawn))
  (Variables|Default|SetBaseTank _asbase_tank))

(fn ConstructionScript)

(fn GetShotMontageTime
  (bind _basetank (Variables|Default|GetBaseTank))
  (bind _basetank_2 (Variables|Default|GetBaseTank))
  (bind _basetank_3 (Variables|Default|GetBaseTank))
  (bind (_asbp_dynamite_adam _bsuccess) (Utilities|Casting|CastToBP_Dynamite_Adam _basetank))
  (bind (_asbp_scrapper_pumpkin _bsuccess_2) (Utilities|Casting|CastToBP_Scrapper_Pumpkin _basetank_2))
  (bind (_asbp_marguerite_lily _bsuccess_3) (Utilities|Casting|CastToBP_Marguerite_Lily _basetank_3))
  ;[1 1 1] Play the correct anim montage and return the time of it
  (if _bsuccess_2
    (bind _returnvalue (Animation|PlayAnimMontage _asbp_scrapper_pumpkin "/Game/Blueprints/Characters/Scrappers/AM_ScrapperShoot.AM_ScrapperShoot" 1.0 "None"))
    (return _returnvalue)
    (elif _bsuccess_3
      (bind _returnvalue_2 (Animation|PlayAnimMontage _asbp_marguerite_lily "/Game/Blueprints/Characters/Marguerite/AM_MargueriteShoot.AM_MargueriteShoot" 1.0 "None"))
      (return _returnvalue_2)
      (elif _bsuccess
        (bind _returnvalue_3 (Animation|PlayAnimMontage _asbp_dynamite_adam "/Game/Blueprints/Characters/Dynamite/AM_DynamiteShoot.AM_DynamiteShoot" 1.0 "None"))
        (return _returnvalue_3)
        (else
          (return 0.0))))))

(fn SpawnProjectile
  (bind _basetank (Variables|Default|GetBaseTank))
  (bind _projectilespawncomponent (Variables|/Script/CartoonTanks.BaseTank|GetProjectileSpawnComponent _basetank))
  ;[1 1 1] Handle spawning the projectile
  (Game|SpawnActorfromClass (Variables|/Script/CartoonTanks.BaseTank|GetProjectileClass _basetank) (Math|Transform|MakeTransform (Transformation|GetWorldLocation _projectilespawncomponent) (Transformation|GetWorldRotation _projectilespawncomponent)) "Undefined" "MultiplyWithRoot" (Variables|Default|GetBaseTank) 0)
  (return))